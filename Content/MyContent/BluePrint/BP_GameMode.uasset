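; Game mode that manages stage progression through level streaming, loading numbered "Stage" sublevels alongside a shared GoalArea level.
; BeginPlay loads the stage number stored in BP_GameInstance.
; NextStage and StageReset clear gimmick flags, unload both levels, destroy all BP_Ball actors, stream in the next or same stage, and respawn BP_Player.
; NextStage also increments the saved stage number.
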(event `self.ReceiveTick`
  (params (DeltaSeconds :type "Float (single-precision)")))

(event `self.ReceiveBeginPlay`
  (`self.Set Stage`))

(event `Set Stage`
  (bind _asbp_game_instance (cast `/Game/MyContent/BluePrint/BP_GameInstance` (`GameplayStatics.GetGameInstance`)))
  (`GameplayStatics.LoadStreamLevel` (`KismetStringLibrary.Conv_StringToName` (`KismetTextLibrary.Conv_TextToString` (`|FormatText` "Stage{1}" (`/Game/MyContent/BluePrint/BP_GameInstance.Stage` _asbp_game_instance)))) true true)
  (`GameplayStatics.LoadStreamLevelBySoftObjectPtr` "/Game/MyContent/Level/Stages/GoalArea.GoalArea" true true))

(event `NextStage`
  (bind _asbp_game_instance (cast `/Game/MyContent/BluePrint/BP_GameInstance` (`GameplayStatics.GetGameInstance`)))
  (set `/Game/MyContent/BluePrint/BP_GameInstance.GimmickFlags` 0 _asbp_game_instance)
  (bind _stage (`/Game/MyContent/BluePrint/BP_GameInstance.Stage` _asbp_game_instance))
  (`GameplayStatics.UnloadStreamLevel` (`KismetStringLibrary.Conv_StringToName` (`KismetTextLibrary.Conv_TextToString` (`|FormatText` "Stage{1}" _stage))))
  (`GameplayStatics.UnloadStreamLevelBySoftObjectPtr` "/Game/MyContent/Level/Stages/GoalArea.GoalArea" true)
  (bind _outactors (`GameplayStatics.GetAllActorsOfClass` "/Game/MyContent/BluePrint/BP_Ball.BP_Ball_C"))
  (for _array_element _outactors
    (`self.K2_DestroyActor` _array_element))
  (bind _returnvalue (+ _stage 1))
  (`GameplayStatics.LoadStreamLevel` (`KismetStringLibrary.Conv_StringToName` (`KismetTextLibrary.Conv_TextToString` (`|FormatText` "Stage{1}" _returnvalue))) true)
  (`GameplayStatics.LoadStreamLevelBySoftObjectPtr` "/Game/MyContent/Level/Stages/GoalArea.GoalArea" true true)
  (bind _asbp_player (cast `/Game/MyContent/BluePrint/BP_Player` (`GameplayStatics.GetPlayerCharacter` 0)))
  (`/Game/MyContent/BluePrint/BP_Player.Respawn` _asbp_player)
  (set `/Game/MyContent/BluePrint/BP_GameInstance.Stage` _returnvalue _asbp_game_instance))

(event `StageReset`
  (bind _asbp_game_instance (cast `/Game/MyContent/BluePrint/BP_GameInstance` (`GameplayStatics.GetGameInstance`)))
  (set `/Game/MyContent/BluePrint/BP_GameInstance.GimmickFlags` 0 _asbp_game_instance)
  (bind _returnvalue (`KismetStringLibrary.Conv_StringToName` (`KismetTextLibrary.Conv_TextToString` (`|FormatText` "Stage{1}" (`/Game/MyContent/BluePrint/BP_GameInstance.Stage` _asbp_game_instance)))))
  (`GameplayStatics.UnloadStreamLevel` _returnvalue true)
  (`GameplayStatics.UnloadStreamLevelBySoftObjectPtr` "/Game/MyContent/Level/Stages/GoalArea.GoalArea" true)
  (bind _outactors (`GameplayStatics.GetAllActorsOfClass` "/Game/MyContent/BluePrint/BP_Ball.BP_Ball_C"))
  (for _array_element _outactors
    (`self.K2_DestroyActor` _array_element))
  (`GameplayStatics.LoadStreamLevel` _returnvalue true true)
  (`GameplayStatics.LoadStreamLevelBySoftObjectPtr` "/Game/MyContent/Level/Stages/GoalArea.GoalArea" true true)
  (bind _asbp_player (cast `/Game/MyContent/BluePrint/BP_Player` (`GameplayStatics.GetPlayerCharacter` 0)))
  (`/Game/MyContent/BluePrint/BP_Player.Respawn` _asbp_player))

(fn `UserConstructionScript`)