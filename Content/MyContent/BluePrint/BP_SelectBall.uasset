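; BP_SelectBall is a ball actor that reacts to being hit by starting a screen transition sequence.
; Its Hited event disables input on BP_Player, waits briefly, then creates and plays the FadeIn level sequence.
; Tick only casts the player character to BP_Player without using it, and the construction script adds nothing beyond the parent call.
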(event `self.ReceiveTick`
  (params (DeltaSeconds :type "Float (single-precision)"))
  (`parent.ReceiveTick` DeltaSeconds)
  (cast `/Game/MyContent/BluePrint/BP_Player` (`GameplayStatics.GetPlayerCharacter` 0)))

(event `Hited`
  (`self.DisableInput` (cast `/Game/MyContent/BluePrint/BP_Player` (`GameplayStatics.GetPlayerCharacter` 0) :!pure true) (`GameplayStatics.GetPlayerController` 0))
  (`KismetSystemLibrary.Delay` 1.0)
  (bind _outactor (`LevelSequencePlayer.CreateLevelSequencePlayer` "/Game/MyContent/Level/StageSelect/FadeIn.FadeIn"))
  (`MovieSceneSequencePlayer.Play` (`LevelSequenceActor.SequencePlayer` _outactor)))

(fn `UserConstructionScript`
  (`parent.UserConstructionScript`))