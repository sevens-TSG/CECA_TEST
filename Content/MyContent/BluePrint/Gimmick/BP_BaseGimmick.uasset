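; BP_BaseGimmick is a base Blueprint for gimmicks whose state depends on other gimmicks' on/off flags.
; GetGimmick looks up each entry in the ID list through BP_GameInstance's IsGimmickOn and returns a combined boolean.
; The And flag selects whether all listed gimmicks must be on or any one suffices.
; Its event graph and construction script hold no logic.
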(fn `GetGimmick`
  (returns (return :type Boolean))
  (locals (ret :type Boolean))
  (bind _id (`self.ID`))
  (bind _asbp_game_instance (cast `/Game/MyContent/BluePrint/BP_GameInstance` (`GameplayStatics.GetGameInstance`)))
  (if (`self.And`)
    (set `local.ret` true)
    (for _array_element _id
      (bind _return (`/Game/MyContent/BluePrint/BP_GameInstance.IsGimmickOn` _asbp_game_instance _array_element))
      (if (not _return)
        (set `local.ret` false)))
    (else
      (for _array_element_2 _id
        (bind _return_2 (`/Game/MyContent/BluePrint/BP_GameInstance.IsGimmickOn` _asbp_game_instance _array_element_2))
        (if _return_2
          (set `local.ret` true)))))
  (return (`local.ret`)))

(fn `UserConstructionScript`)