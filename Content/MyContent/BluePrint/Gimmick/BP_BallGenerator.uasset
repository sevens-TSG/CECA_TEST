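; BP_BallGenerator is a gimmick actor that spawns a BP_Ball at its own transform on BeginPlay and replaces it when needed.
; It keeps a reference to the current ball, marks it respawnable, and polls its ReSpawn flag every Tick.
; When the flag is set, it destroys the ball, spawns a new one and launches it along the Arrow component's forward direction with a strong force.
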(event `self.ReceiveBeginPlay`
  (`parent.ReceiveBeginPlay`)
  (bind _returnvalue (`|SpawnActorFromClass` "/Game/MyContent/BluePrint/BP_Ball.BP_Ball_C" (`self.GetTransform`) "Undefined" "OverrideRootScale" null null))
  (bind _output_get (set `self.Ball` _returnvalue))
  (set `/Game/MyContent/BluePrint/BP_Ball.CanRespawn` true _output_get))

(event `self.ReceiveTick`
  (params (DeltaSeconds :type "Float (single-precision)"))
  (bind _ball (`self.Ball`))
  (`parent.ReceiveTick` DeltaSeconds)
  (if (`/Game/MyContent/BluePrint/BP_Ball.ReSpawn` _ball)
    (`self.K2_DestroyActor` _ball)
    (bind _returnvalue (`|SpawnActorFromClass` "/Game/MyContent/BluePrint/BP_Ball.BP_Ball_C" (`self.GetTransform`) "Undefined" "OverrideRootScale" null null))
    (`PrimitiveComponent.AddForce` (`/Game/MyContent/BluePrint/BP_Ball.Sphere` _returnvalue) (* (`KismetMathLibrary.GetForwardVector` (`SceneComponent.K2_GetComponentRotation` (`self.Arrow`))) 400000.0) "None" false)
    (bind _output_get (set `self.Ball` _returnvalue))
    (set `/Game/MyContent/BluePrint/BP_Ball.CanRespawn` true _output_get)))

(fn `UserConstructionScript`
  (`parent.UserConstructionScript`))