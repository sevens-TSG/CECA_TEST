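; BP_BrakeWall is a breakable wall gimmick that shatters when a BP_Ball hits it, using a Destructible component.
; A ball hit applies damage with an impulse pointing from the ball toward the wall.
; With Penetrate set, the wall's collision is off from start and a Box overlap triggers the break instead.
; On fracture, collision turns off and a timeline drives the material's alpha parameter before destroying the actor.
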(event `self.ReceiveBeginPlay`
  (if (`self.penetrate`)
    (`PrimitiveComponent.SetCollisionEnabled` (`self.Destructible`) "NoCollision")))

(event `self.Destructible.OnComponentHit`
  (params (HitComponent :type "PrimitiveComponent Object Reference") (OtherActor :type "Actor Object Reference") (OtherComp :type "PrimitiveComponent Object Reference") (NormalImpulse :type "Vector Structure") (Hit :type "HitResult Structure (by ref)"))
  (bind _destructible (`self.Destructible`))
  (bind _returnvalue (`SceneComponent.K2_GetComponentLocation` _destructible))
  (bind _asbp_ball (cast `/Game/MyContent/BluePrint/BP_Ball` OtherActor))
  (bind _sphere (`/Game/MyContent/BluePrint/BP_Ball.Sphere` _asbp_ball))
  (`PrimitiveComponent.GetPhysicsLinearVelocity` _sphere "None")
  (`DestructibleComponent.ApplyDamage` _destructible 1000.0 _returnvalue (`KismetMathLibrary.GetForwardVector` (`KismetMathLibrary.FindLookAtRotation` (`SceneComponent.K2_GetComponentLocation` _sphere) _returnvalue)) 50000.0))

(event `self.Destructible.OnComponentFracture`
  (params (HitPoint :type "Vector Structure (by ref)") (HitDirection :type "Vector Structure (by ref)"))
  (bind _destructible (`self.Destructible`))
  (`PrimitiveComponent.SetCollisionEnabled` _destructible "NoCollision")
  (`PrimitiveComponent.CreateDynamicMaterialInstance` _destructible 0 "/Game/MyContent/Material/M_Debug.M_Debug" "None")
  (bind (_direction _alpha) (`Timeline|タイムライン_0`)
    (:`Update`
      (`MeshComponent.SetScalarParameterValueOnMaterials` _destructible "alpha" _alpha))
    (:`Finished`
      (`self.K2_DestroyActor`))))

(event `self.Box.OnComponentBeginOverlap`
  (params (OverlappedComponent :type "PrimitiveComponent Object Reference") (OtherActor :type "Actor Object Reference") (OtherComp :type "PrimitiveComponent Object Reference") (OtherBodyIndex :type Integer) (bFromSweep :type Boolean) (SweepResult :type "HitResult Structure (by ref)"))
  (bind _destructible (`self.Destructible`))
  (bind _returnvalue (`SceneComponent.K2_GetComponentLocation` _destructible))
  (if (`self.penetrate`)
    (bind _asbp_ball (cast `/Game/MyContent/BluePrint/BP_Ball` OtherActor))
    (bind _sphere (`/Game/MyContent/BluePrint/BP_Ball.Sphere` _asbp_ball))
    (`PrimitiveComponent.GetPhysicsLinearVelocity` _sphere "None")
    (`DestructibleComponent.ApplyDamage` _destructible 1000.0 _returnvalue (`KismetMathLibrary.GetForwardVector` (`KismetMathLibrary.FindLookAtRotation` (`SceneComponent.K2_GetComponentLocation` _sphere) _returnvalue)) 50000.0)))

(fn `UserConstructionScript`)