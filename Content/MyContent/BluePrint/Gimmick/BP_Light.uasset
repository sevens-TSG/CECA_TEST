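; BP_Light is a gimmick indicator light that switches between red and green to reflect a gimmick state.
; Every tick it reads GetGimmick, hiding the red light and showing the green one when true, and the reverse when false.
; It also flips the Mode scalar on the sphere's dynamic M_Light material, created at BeginPlay, to match that state.
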(event `self.ReceiveBeginPlay`
  (`parent.ReceiveBeginPlay`)
  (`PrimitiveComponent.CreateDynamicMaterialInstance` (`self.Sphere`) 0 "/Game/MyContent/Model/M_Light.M_Light" "None"))

(event `self.ReceiveTick`
  (params (DeltaSeconds :type "Float (single-precision)"))
  (bind _sphere (`self.Sphere`))
  (`parent.ReceiveTick` DeltaSeconds)
  (bind _return (`self.GetGimmick`))
  (`SceneComponent.SetHiddenInGame` (`self.RedLight`) _return false)
  (`SceneComponent.SetHiddenInGame` (`self.GreenLight`) (not _return) false)
  (if _return
    (`MeshComponent.SetScalarParameterValueOnMaterials` _sphere "Mode" -1.0)
    (else
      (`MeshComponent.SetScalarParameterValueOnMaterials` _sphere "Mode" 1.0))))

(fn `UserConstructionScript`
  (`parent.UserConstructionScript`))