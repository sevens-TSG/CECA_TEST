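; BP_GateBlock is a gimmick gate block that rises to open when its gimmick flag is set.
; Each Tick it checks GetGimmick and, while true, moves the Cube up by a fixed world offset, with no sweep, delta-time scaling or upper limit.
; A DoOnce plays the gate-open sound at the root's location on the first rising frame.
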(event `self.ReceiveTick`
  (params (DeltaSeconds :type "Float (single-precision)"))
  (`parent.ReceiveTick` DeltaSeconds)
  (bind _return (`self.GetGimmick`))
  (if _return
    (`SceneComponent.K2_AddWorldOffset` (`self.Cube`) (0.0 0.0 20.0) false false)
    (`/Engine/EditorBlueprintResources/StandardMacros.DoOnce` false
      (:`Completed`
        (`GameplayStatics.PlaySoundAtLocation` "/Game/MyContent/Sounds/SE_GateOpen.SE_GateOpen" (`SceneComponent.K2_GetComponentLocation` (`self.DefaultSceneRoot`)) (struct) 1.0 1.0 0.0 null null null)))))

(fn `UserConstructionScript`
  (`parent.UserConstructionScript`))