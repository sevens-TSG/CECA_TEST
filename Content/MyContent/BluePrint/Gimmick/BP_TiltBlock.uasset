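; BP_TiltBlock is a gimmick block that tilts its Cube left, right, front or back when triggered through gimmick IDs.
; Each Tick, it polls BP_GameInstance for four IDs, clearing any active one.
; A trigger sets a signed pitch or roll target, or levels that axis if tilted the opposite way.
; Comper steps the current angles one unit per frame toward their targets, independent of delta time.
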(event `self.ReceiveTick`
  (params (DeltaSeconds :type "Float (single-precision)"))
  (bind _pitch (`self.Pitch`))
  (bind _roll (`self.Roll`))
  (`parent.ReceiveTick` DeltaSeconds)
  (bind _asbp_game_instance (cast `/Game/MyContent/BluePrint/BP_GameInstance` (`GameplayStatics.GetGameInstance`)))
  (`|ExecutionSequence`
    (:`then_0`
      (bind _ret (`self.Comper` _pitch (`self.TargetPitch`)))
      (switch `int` _ret
        (:`Default`
          _)
        (:`0`
          (`/Engine/EditorBlueprintResources/StandardMacros.DecrementFloat` _pitch
            (:`  `
              _)))
        (:`1`
          (`/Engine/EditorBlueprintResources/StandardMacros.IncrementFloat` _pitch
            (:`  `
              _))))
      (bind _ret_2 (`self.Comper` _roll (`self.TargetRoll`)))
      (switch `int` _ret_2
        (:`Default`
          _)
        (:`0`
          (`/Engine/EditorBlueprintResources/StandardMacros.DecrementFloat` _roll
            (:`  `
              _)))
        (:`1`
          (`/Engine/EditorBlueprintResources/StandardMacros.IncrementFloat` _roll
            (:`  `
              _))))
      (`SceneComponent.K2_SetRelativeRotation` (`self.Cube`) (`KismetMathLibrary.MakeRotator` (`self.Roll`) (`self.Pitch`)) false false))
    (:`then_1`
      (bind _ret_3 (`self.Chack` _asbp_game_instance (`self.ID_LEFT`)))
      (if _ret_3
        (if (`self.TiltFlag_RIGHT`)
          (set `self.TiltFlag_RIGHT` false)
          (set `self.TargetPitch` 0.0)
          (else
            (set `self.TiltFlag_LEFT` true)
            (set `self.TargetPitch` (`self.Rot`))))))
    (:`then_2`
      (bind _ret_4 (`self.Chack` _asbp_game_instance (`self.ID_RIGHT`)))
      (if _ret_4
        (if (`self.TiltFlag_LEFT`)
          (set `self.TiltFlag_LEFT` false)
          (set `self.TargetPitch` 0.0)
          (else
            (set `self.TiltFlag_RIGHT` true)
            (set `self.TargetPitch` (* -1 (`self.Rot`)))))))
    (:`then_3`
      (bind _ret_5 (`self.Chack` _asbp_game_instance (`self.ID_FRONT`)))
      (if _ret_5
        (if (`self.TiltFlag_BACK`)
          (set `self.TiltFlag_BACK` false)
          (set `self.TargetRoll` 0.0)
          (else
            (set `self.TiltFlag_FRONT` true)
            (set `self.TargetRoll` (`self.Rot`))))))
    (:`then_4`
      (bind _ret_6 (`self.Chack` _asbp_game_instance (`self.ID_BACK`)))
      (if _ret_6
        (if (`self.TiltFlag_FRONT`)
          (set `self.TiltFlag_FRONT` false)
          (set `self.TargetRoll` 0.0)
          (else
            (set `self.TiltFlag_BACK` true)
            (set `self.TargetRoll` (* -1 (`self.Rot`)))))))))

(fn `Chack`
  (params (GameInstance :type "/Game/MyContent/BluePrint/BP_GameInstance Object Reference") (ID :type Integer))
  (returns (ret :type Boolean))
  (bind _return (`/Game/MyContent/BluePrint/BP_GameInstance.IsGimmickOn` GameInstance ID))
  (if _return
    (`/Game/MyContent/BluePrint/BP_GameInstance.GimmickOff` GameInstance ID)
    (return true)
    (else
      (return false))))

(fn `Comper`
  (params (in :type "Float (double-precision)") (Comp :type "Float (double-precision)"))
  (returns (ret :type Integer))
  (if (> in Comp)
    (return 0)
    (elif (< in Comp)
      (return 1)
      (else
        (return 2)))))

(fn `UserConstructionScript`
  (`parent.UserConstructionScript`))