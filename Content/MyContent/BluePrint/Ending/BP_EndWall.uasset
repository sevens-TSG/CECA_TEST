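; BP_EndWall is a breakable wall actor in the Ending content that displays a text label and shatters when a BP_Ball hits it.
; BeginPlay copies the Text variable onto the TextRender component.
; A ball hit applies damage to the Destructible component with a strong impulse directed from the ball toward the wall.
; On fracture, the wall disables its collision and hides the text.
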(event `self.ReceiveBeginPlay`
  (`TextRenderComponent.K2_SetText` (`self.TextRender`) (`self.Text`)))

(event `self.Destructible1.OnComponentHit`
  (params (HitComponent :type "PrimitiveComponent Object Reference") (OtherActor :type "Actor Object Reference") (OtherComp :type "PrimitiveComponent Object Reference") (NormalImpulse :type "Vector Structure") (Hit :type "HitResult Structure (by ref)"))
  (bind _destructible1 (`self.Destructible1`))
  (bind _returnvalue (`SceneComponent.K2_GetComponentLocation` _destructible1))
  (bind _asbp_ball (cast `/Game/MyContent/BluePrint/BP_Ball` OtherActor))
  (`DestructibleComponent.ApplyDamage` _destructible1 1.0 _returnvalue (`KismetMathLibrary.GetForwardVector` (`KismetMathLibrary.FindLookAtRotation` (`SceneComponent.K2_GetComponentLocation` (`/Game/MyContent/BluePrint/BP_Ball.Sphere` _asbp_ball)) _returnvalue)) 1000000.0))

(event `self.Destructible1.OnComponentFracture`
  (params (HitPoint :type "Vector Structure (by ref)") (HitDirection :type "Vector Structure (by ref)"))
  (`PrimitiveComponent.SetCollisionEnabled` (`self.Destructible1`) "NoCollision")
  (`SceneComponent.SetHiddenInGame` (`self.TextRender`) true false))

(fn `UserConstructionScript`)