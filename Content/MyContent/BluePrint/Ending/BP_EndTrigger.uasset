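; BP_EndTrigger is a box trigger in the Ending folder that sends the player back through respawn behind a fade.
; When BP_Player overlaps the box, it plays the Fade sequence, then calls Respawn on the player twice, with a delay before each call.
; It then calls BreakObjectLoad on BP_GameMode and destroys itself after a final player-character cast check.
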(event `self.ReceiveTick`
  (params (DeltaSeconds :type "Float (single-precision)")))

(event `self.Box.OnComponentBeginOverlap`
  (params (OverlappedComponent :type "PrimitiveComponent Object Reference") (OtherActor :type "Actor Object Reference") (OtherComp :type "PrimitiveComponent Object Reference") (OtherBodyIndex :type Integer) (bFromSweep :type Boolean) (SweepResult :type "HitResult Structure (by ref)"))
  (bind _asbp_player (cast `/Game/MyContent/BluePrint/BP_Player` OtherActor))
  (`MovieSceneSequencePlayer.Play` (`LevelSequenceActor.SequencePlayer` (`self.Fade`)))
  (`KismetSystemLibrary.Delay` 3.0)
  (`/Game/MyContent/BluePrint/BP_Player.Respawn` _asbp_player)
  (`KismetSystemLibrary.Delay` 1.0)
  (`/Game/MyContent/BluePrint/BP_Player.Respawn` _asbp_player)
  (bind _asbp_game_mode (cast `/Game/MyContent/BluePrint/BP_GameMode` (`GameplayStatics.GetGameMode`)))
  (`/Game/MyContent/BluePrint/BP_GameMode.BreakObjectLoad` _asbp_game_mode)
  (cast `/Game/MyContent/BluePrint/BP_Player` (`GameplayStatics.GetPlayerCharacter` 0))
  (`self.K2_DestroyActor`))

(fn `UserConstructionScript`)