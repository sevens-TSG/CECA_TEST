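; BP_GameStart is a destructible title object that starts the game when a BP_Ball hits it, moving on to the StageSelect level.
; On component hit, it applies damage with a strong impulse directed from the ball's sphere toward the destructible's location.
; It then plays a level sequence and opens the stage select level after a short delay.
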(event `self.Destructible.OnComponentHit`
  (params (HitComponent :type "PrimitiveComponent Object Reference") (OtherActor :type "Actor Object Reference") (OtherComp :type "PrimitiveComponent Object Reference") (NormalImpulse :type "Vector Structure") (Hit :type "HitResult Structure (by ref)"))
  (bind _destructible (`self.Destructible`))
  (bind _returnvalue (`SceneComponent.K2_GetComponentLocation` _destructible))
  (bind _asbp_ball (cast `/Game/MyContent/BluePrint/BP_Ball` OtherActor))
  (`DestructibleComponent.ApplyDamage` _destructible 1.0 _returnvalue (`KismetMathLibrary.GetForwardVector` (`KismetMathLibrary.FindLookAtRotation` (`SceneComponent.K2_GetComponentLocation` (`/Game/MyContent/BluePrint/BP_Ball.Sphere` _asbp_ball)) _returnvalue)) 50000.0)
  (`MovieSceneSequencePlayer.Play` (`LevelSequenceActor.SequencePlayer` (`self.Sequence`)))
  (`KismetSystemLibrary.Delay` 2.0)
  (`GameplayStatics.OpenLevelBySoftObjectPtr` "/Game/MyContent/Level/StageSelect/StageSelect.StageSelect"))

(fn `UserConstructionScript`)