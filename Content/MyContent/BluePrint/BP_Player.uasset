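; Player character that smashes balls toward targets, respawns below Z=0, and shows a clear UI on reaching a goal.
; Left-stick movement snaps to digital axes and stops while swinging or charging.
; Mouse hold-and-flick or right-stick charge-and-release builds Power for BallSmash.
; BallSmash launches balls inside SmashBox at the nearest SearchBox-flagged target, else along SmashVector, with camera shake and time-dilation hit stop.
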(event `self.SearchBox.OnComponentBeginOverlap`
  (params (OverlappedComponent :type "PrimitiveComponent Object Reference") (OtherActor :type "Actor Object Reference") (OtherComp :type "PrimitiveComponent Object Reference") (OtherBodyIndex :type Integer) (bFromSweep :type Boolean) (SweepResult :type "HitResult Structure (by ref)"))
  ;[1 1 1] Target
  (bind _asbp_base_target (cast `/Game/MyContent/BluePrint/Target/BP_BaseTarget` OtherActor))
  (if (`/Game/MyContent/BluePrint/Target/BP_BaseTarget.CanTarget` _asbp_base_target)
    (set `/Game/MyContent/BluePrint/Target/BP_BaseTarget.Targeted` true _asbp_base_target)))

(event `InputAxis|L_Y`
  (params (AxisValue :type "Float (single-precision)"))
  (bind (_returnvalue_roll _returnvalue_pitch _returnvalue_yaw) (`KismetMathLibrary.BreakRotator` (`self.GetControlRotation`)))
  (bind _returnvalue (`KismetMathLibrary.ClampVectorSize` (`KismetMathLibrary.MakeVector` (`self.SetAxis` (`self.GetInputAxisValue`)) (`self.SetAxis` (`self.GetInputAxisValue`))) 0.0 1.0))
  ;[1 1 1] Move
  (if (not (or (`self.SwingFlag`) (`self.ChargeFlag`) (`self.CantMove`)))
    (`self.AddMovementInput` (`KismetMathLibrary.GetForwardVector` (`KismetMathLibrary.MakeRotator` 0.0 0.0 _returnvalue_yaw)) (`self.SetAxis` AxisValue))
    (if (> (`KismetMathLibrary.VSize` _returnvalue) 0.0) :!label _label
      (`SceneComponent.K2_SetWorldRotation` (`self.Mesh`) (`KismetMathLibrary.Conv_VectorToRotator` _returnvalue) false false))))

(event `self.ReceiveTick`
  (params (DeltaSeconds :type "Float (single-precision)"))
  (bind (_returnvalue_x _returnvalue_y _returnvalue_z) (`KismetMathLibrary.BreakVector` (`self.K2_GetActorLocation`)))
  ;[1 1 1] Tick
  (set `self.CoolTime` (- (`self.CoolTime`) DeltaSeconds))
  (`self.Swing`)
  (`self.Charge`)
  (if (< _returnvalue_z 0.0)
    (`self.Respawn`)))

(event `self.SearchBox.OnComponentEndOverlap`
  (params (OverlappedComponent :type "PrimitiveComponent Object Reference") (OtherActor :type "Actor Object Reference") (OtherComp :type "PrimitiveComponent Object Reference") (OtherBodyIndex :type Integer))
  ;[1 1 1] Target
  (bind _asbp_base_target (cast `/Game/MyContent/BluePrint/Target/BP_BaseTarget` OtherActor))
  (set `/Game/MyContent/BluePrint/Target/BP_BaseTarget.Targeted` false _asbp_base_target))

(event `InputAxis|L_X`
  (params (AxisValue :type "Float (single-precision)"))
  (bind (_returnvalue_roll _returnvalue_pitch _returnvalue_yaw) (`KismetMathLibrary.BreakRotator` (`self.GetControlRotation`)))
  ;[1 1 1] Move
  (if (not (or (`self.SwingFlag`) (`self.ChargeFlag`) (`self.CantMove`)))
    (`self.AddMovementInput` (`KismetMathLibrary.GetRightVector` (`KismetMathLibrary.MakeRotator` 0.0 0.0 _returnvalue_yaw)) (`self.SetAxis` AxisValue))
    (goto _label)))

(event `SetTarget`
  (bind (_returnvalue_x _returnvalue_y) (`KismetMathLibrary.BreakVector` (`SceneComponent.K2_GetComponentLocation` (`self.SmashVector`))))
  (bind _returnvalue (`KismetMathLibrary.MakeVector` _returnvalue_x _returnvalue_y))
  ;[1 1 1] Target
  (set `self.TargetFlag` false)
  (bind _outactors (`GameplayStatics.GetAllActorsOfClass` "/Game/MyContent/BluePrint/Target/BP_BaseTarget.BP_BaseTarget_C"))
  (for _array_element _outactors
    (if (`/Game/MyContent/BluePrint/Target/BP_BaseTarget.Targeted` _array_element)
      (bind _pos (`/Game/MyContent/BluePrint/Target/BP_BaseTarget.GetPosition` _array_element))
      (bind _returnvalue_2 (`KismetMathLibrary.MakeVector` (.x _pos) (.y _pos)))
      (if (< (`KismetMathLibrary.VSize` (- _returnvalue_2 _returnvalue)) (`KismetMathLibrary.VSize` (- (`self.TargetPos`) _returnvalue)))
        (set `self.TargetPos` _returnvalue_2 :!label _label_2)
        (set `self.TargetFlag` true)
        (elif (not (`self.TargetFlag`))
          (goto _label_2))))))

(event `self.SmashBox.OnComponentBeginOverlap`
  (params (OverlappedComponent :type "PrimitiveComponent Object Reference") (OtherActor :type "Actor Object Reference") (OtherComp :type "PrimitiveComponent Object Reference") (OtherBodyIndex :type Integer) (bFromSweep :type Boolean) (SweepResult :type "HitResult Structure (by ref)"))
  ;[1 1 1] BallBox
  (bind _asbp_ball (cast `/Game/MyContent/BluePrint/BP_Ball` OtherActor))
  (set `/Game/MyContent/BluePrint/BP_Ball.CanSmash` true _asbp_ball))

(event `InputAction|MouseL`
  (params (Key :type "Key Structure"))
  ;[1 1 1] Mouse
  (:`Pressed`
    (set `self.SwingFlag` true))
  (:`Released`
    (set `self.SwingFlag` false)
    (set `self.Power` 0.0)))

(event `self.ReceiveBeginPlay`
  ;[1 1 1] Init
  (set `self.RespawnLocation` (`self.K2_GetActorLocation`)))

(event `self.SmashBox.OnComponentEndOverlap`
  (params (OverlappedComponent :type "PrimitiveComponent Object Reference") (OtherActor :type "Actor Object Reference") (OtherComp :type "PrimitiveComponent Object Reference") (OtherBodyIndex :type Integer))
  ;[1 1 1] BallBox
  (bind _asbp_ball (cast `/Game/MyContent/BluePrint/BP_Ball` OtherActor))
  (set `/Game/MyContent/BluePrint/BP_Ball.CanSmash` false _asbp_ball))

(event `self.Sphere1.OnComponentBeginOverlap`
  (params (OverlappedComponent :type "PrimitiveComponent Object Reference") (OtherActor :type "Actor Object Reference") (OtherComp :type "PrimitiveComponent Object Reference") (OtherBodyIndex :type Integer) (bFromSweep :type Boolean) (SweepResult :type "HitResult Structure (by ref)"))
  (bind _returnvalue (`GameplayStatics.GetPlayerController` 0))
  ;[1 1 1] Goal
  (cast `/Game/MyContent/BluePrint/BP_Goal` OtherActor)
  (cast `/Game/MyContent/BluePrint/BP_GameMode` (`GameplayStatics.GetGameMode`))
  (bind _returnvalue_2 (`|CreateWidget` "/Game/MyContent/BluePrint/BP_PlayClearUI.BP_PlayClearUI_C"))
  (`UserWidget.AddToViewport` _returnvalue_2 0)
  (`WidgetBlueprintLibrary.SetInputMode_GameAndUIEx` _returnvalue _returnvalue_2 "DoNotLock" false)
  (set `PlayerController.bShowMouseCursor` true _returnvalue)
  (set `self.CantMove` true))

(event `Swing`
  ;[1 1 1] Swing
  (if (`self.SwingFlag`)
    (if (< (`self.GetInputAxisKeyValue`) -2.0)
      (set `self.SwingFlag` false)
      (`self.BallSmash`)
      (set `self.Power` 0.0)
      (else
        (bind _output_get (set `self.Power` (`KismetMathLibrary.FClamp` (+ (`self.Power`) 0.01))))
        (`KismetSystemLibrary.PrintString` (`KismetStringLibrary.Conv_DoubleToString` _output_get) true true (struct :`G` 0.66 :`B` 1.0 :`A` 1.0) 0.0)))))

(event `BallSmash`
  ;[1 1 1] BallSmash
  (`self.SetTarget`)
  (bind _outactors (`GameplayStatics.GetAllActorsOfClass` "/Game/MyContent/BluePrint/BP_Ball.BP_Ball_C"))
  (for _array_element _outactors
    (if (`/Game/MyContent/BluePrint/BP_Ball.CanSmash` _array_element)
      (if (`self.TargetFlag`)
        (bind _sphere (`/Game/MyContent/BluePrint/BP_Ball.Sphere` _array_element))
        (`PrimitiveComponent.AddForce` _sphere (* (`KismetMathLibrary.GetForwardVector` (`KismetMathLibrary.FindLookAtRotation` (`SceneComponent.K2_GetComponentLocation` _sphere) (`self.TargetPos`))) (* (`KismetMathLibrary.MultiplyMultiply_FloatFloat` 10.0 5.0) (* (`self.Power`) 5.0))) "None" true)
        (else
          (`PrimitiveComponent.AddForce` _sphere (* (`KismetMathLibrary.GetForwardVector` (`SceneComponent.K2_GetComponentRotation` (`self.SmashVector`))) (* (`KismetMathLibrary.MultiplyMultiply_FloatFloat` 10.0 5.0) (* (`self.Power`) 5.0))) "None" true)))
      (`PlayerController.ClientStartCameraShake` :`self` (`GameplayStatics.GetPlayerController` 0) :`Shake` "/Game/MyContent/BluePrint/BP_CameraShake.BP_CameraShake_C")
      (set `self.StopFlag` true)
      (bind _asbp_select_ball (cast `/Game/MyContent/BluePrint/BP_SelectBall` _array_element))
      (`/Game/MyContent/BluePrint/BP_SelectBall.Hited` _asbp_select_ball)))
  (if (`self.StopFlag`)
    (`GameplayStatics.SetGlobalTimeDilation` 0.01)
    (`KismetSystemLibrary.Delay` 0.02)
    (`GameplayStatics.SetGlobalTimeDilation` 1.0)
    (set `self.StopFlag` false)))

(event `Respawn`
  ;[1 1 1] Respawn
  (`SceneComponent.K2_SetWorldLocation` (`self.CapsuleComponent`) (`self.RespawnLocation`) false false)
  (set `self.CantMove` false))

(event `Charge`
  (bind _returnvalue (`self.GetInputAxisValue`))
  ;[1 1 1] Charge
  (if (< 0.0 _returnvalue)
    (if (not (`self.ChargeFlag`))
      (set `self.ChargeFlag` true)
      (set `self.Power` 0.0))
    (bind _output_get (set `self.Power` (`KismetMathLibrary.FClamp` (+ (* _returnvalue 0.01) (`self.Power`)))))
    (`KismetSystemLibrary.PrintString` (`KismetStringLibrary.Conv_DoubleToString` _output_get))
    (elif (`self.ChargeFlag`)
      (set `self.ChargeFlag` false)
      (`self.BallSmash`)
      (set `self.Power` 0.0))))

(fn `GetPosition`
  (returns (Pos :type "Vector Structure"))
  (return (`SceneComponent.K2_GetComponentLocation` (`self.CapsuleComponent`))))

(fn `GetRotator`
  (returns (Rot :type "Rotator Structure"))
  (return (`KismetMathLibrary.MakeRotator` 0.0 0.0 (.yaw (`self.GetControlRotation`)))))

(fn `SetAxis`
  (params (In :type "Float (double-precision)"))
  (returns (Out :type "Float (double-precision)"))
  (if (< In -0.3)
    (return -1.0)
    (elif (> In 0.3)
      (return 1.0)
      (else
        (return 0.0)))))

(fn `UserConstructionScript`)