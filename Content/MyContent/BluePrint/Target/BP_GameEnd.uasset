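; BP_GameEnd is the game-ending actor that returns to the Title level when a BP_Ball overlaps its sphere.
; On BeginPlay it caches the level's LevelSequenceActor as Fade and collects every StaticMeshActor whose mesh is named SM_Mannequin.
; The hit enables physics on its own mannequin and the collected ones, clears CanTarget, plays the sequence, then opens Title after a short delay.
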(event `self.ReceiveBeginPlay`
  (`parent.ReceiveBeginPlay`)
  (bind _returnvalue (`GameplayStatics.GetActorOfClass` "/Script/LevelSequence.LevelSequenceActor"))
  (set `self.fade` _returnvalue)
  (bind _outactors (`GameplayStatics.GetAllActorsOfClass` "/Script/Engine.StaticMeshActor"))
  (for _array_element _outactors
    (if (`KismetStringLibrary.EqualEqual_StrStr` (`KismetSystemLibrary.GetObjectName` (`StaticMeshComponent.StaticMesh` (`StaticMeshActor.StaticMeshComponent` _array_element))) "SM_Mannequin")
      (`KismetArrayLibrary.Array_Add` (`self.Mesh`) _array_element))))

(event `self.Sphere.OnComponentBeginOverlap`
  (params (OverlappedComponent :type "PrimitiveComponent Object Reference") (OtherActor :type "Actor Object Reference") (OtherComp :type "PrimitiveComponent Object Reference") (OtherBodyIndex :type Integer) (bFromSweep :type Boolean) (SweepResult :type "HitResult Structure (by ref)"))
  (cast `/Game/MyContent/BluePrint/BP_Ball` OtherActor)
  (`PrimitiveComponent.SetSimulatePhysics` (`self.SM_Mannequin`) true)
  (for _array_element (`self.Mesh`)
    (`PrimitiveComponent.SetSimulatePhysics` (`StaticMeshActor.StaticMeshComponent` _array_element) true))
  (set `self.CanTarget` false)
  (`MovieSceneSequencePlayer.Play` (`LevelSequenceActor.SequencePlayer` (`self.fade`)))
  (`KismetSystemLibrary.Delay` 1.0)
  (`GameplayStatics.OpenLevelBySoftObjectPtr` "/Game/MyContent/Level/Title/Title.Title"))

(fn `UserConstructionScript`
  (`parent.UserConstructionScript`))