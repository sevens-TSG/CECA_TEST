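; BP_FallBall is a ball actor in the Target folder that reports to its gimmick logic once it has fallen out of bounds.
; On BeginPlay it runs the parent logic and turns off CanTarget.
; Each Tick checks the Sphere's world height and, below a fixed negative Z threshold, calls Gimmick with true and destroys the actor.
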(event `self.ReceiveBeginPlay`
  (`parent.ReceiveBeginPlay`)
  (set `self.CanTarget` false))

(event `self.ReceiveTick`
  (params (DeltaSeconds :type "Float (single-precision)"))
  (bind (_returnvalue_x _returnvalue_y _returnvalue_z) (`KismetMathLibrary.BreakVector` (`SceneComponent.K2_GetComponentLocation` (`self.Sphere`))))
  (`parent.ReceiveTick` DeltaSeconds)
  (if (< _returnvalue_z -500.0)
    (`self.Gimmick` true)
    (`self.K2_DestroyActor`)))

(fn `UserConstructionScript`
  (`parent.UserConstructionScript`))