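; Base actor for targetable objects that show a cone marker and can switch gimmicks on or off.
; Each tick, the cone's visibility follows CanTarget and it rotates relative to the player camera, using a look-at rotation with flipped pitch.
; GetPosition exposes the root's world location.
; Gimmick passes an on/off flag for every entry in its ID array to BP_GameInstance.
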(event `self.ReceiveTick`
  (params (DeltaSeconds :type "Float (single-precision)"))
  (bind (_returnvalue_roll _returnvalue_pitch _returnvalue_yaw) (`KismetMathLibrary.BreakRotator` (`KismetMathLibrary.FindLookAtRotation` (`SceneComponent.K2_GetComponentLocation` (`self.Cone`)) (`PlayerCameraManager.GetCameraLocation` (`GameplayStatics.GetPlayerCameraManager` 0)))))
  (`SceneComponent.SetVisibility` (`self.Cone`) (`self.CanTarget`) false)
  (`SceneComponent.K2_SetWorldRotation` (`self.Cone`) (`KismetMathLibrary.MakeRotator` _returnvalue_roll (+ _returnvalue_pitch 180.0) _returnvalue_yaw) false false))

(fn `GetPosition`
  (returns (Pos :type "Vector Structure"))
  (return (`SceneComponent.K2_GetComponentLocation` (`self.DefaultSceneRoot`))))

(fn `Gimmick`
  (params (flag :type Boolean))
  (bind _id (`self.ID`))
  (bind _asbp_game_instance (cast `/Game/MyContent/BluePrint/BP_GameInstance` (`GameplayStatics.GetGameInstance`)))
  (if flag
    (for _array_element _id
      (`/Game/MyContent/BluePrint/BP_GameInstance.GimmickOn` _asbp_game_instance _array_element))
    (else
      (for _array_element_2 _id
        (`/Game/MyContent/BluePrint/BP_GameInstance.GimmickOff` _asbp_game_instance _array_element_2)))))

(fn `UserConstructionScript`)