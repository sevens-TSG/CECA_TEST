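; BP_StageSelect is a destructible target that opens the StageSelect level when a BP_Ball hits it.
; On BeginPlay it finds the LevelSequenceActor named "PlayFade" and stores it as Fade.
; The first ball hit, gated by DoOnce, breaks the Destructible with an impulse directed away from the ball.
; It also spawns an explosion, plays the fade and bomb sound, then loads the level after a short delay.
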(event `self.ReceiveBeginPlay`
  (`parent.ReceiveBeginPlay`)
  (bind _outactors (`GameplayStatics.GetAllActorsOfClass` "/Script/LevelSequence.LevelSequenceActor"))
  (for _array_element _outactors
    (if (`KismetStringLibrary.EqualEqual_StrStr` (`KismetSystemLibrary.GetObjectName` _array_element) "PlayFade")
      (set `self.Fade` _array_element))))

(event `self.Destructible.OnComponentHit`
  (params (HitComponent :type "PrimitiveComponent Object Reference") (OtherActor :type "Actor Object Reference") (OtherComp :type "PrimitiveComponent Object Reference") (NormalImpulse :type "Vector Structure") (Hit :type "HitResult Structure (by ref)"))
  (bind (_returnvalue_location _returnvalue_rotation _returnvalue_scale) (`KismetMathLibrary.BreakTransform` (`self.GetTransform`)))
  (bind _destructible (`self.Destructible`))
  (bind _returnvalue (`SceneComponent.K2_GetComponentLocation` _destructible))
  (bind _asbp_ball (cast `/Game/MyContent/BluePrint/BP_Ball` OtherActor))
  (`/Engine/EditorBlueprintResources/StandardMacros.DoOnce` false
    (:`Completed`
      (`DestructibleComponent.ApplyDamage` _destructible 1.0 _returnvalue (`KismetMathLibrary.GetForwardVector` (`KismetMathLibrary.FindLookAtRotation` (`SceneComponent.K2_GetComponentLocation` (`/Game/MyContent/BluePrint/BP_Ball.Sphere` _asbp_ball)) _returnvalue)) 5000000.0)
      (`GameplayStatics.SpawnEmitterAtLocation` "/Game/StarterContent/Particles/P_Explosion.P_Explosion" _returnvalue_location _returnvalue_rotation (* _returnvalue_scale 10.0))
      (`MovieSceneSequencePlayer.Play` (`LevelSequenceActor.SequencePlayer` (`self.Fade`)))
      (`GameplayStatics.PlaySoundAtLocation` "/Game/MyContent/Sounds/SE_Bomb.SE_Bomb" (`self.K2_GetActorLocation`) (struct) 1.0 1.0 0.0 null null null)
      (`KismetSystemLibrary.Delay` 2.0)
      (`GameplayStatics.OpenLevelBySoftObjectPtr` "/Game/MyContent/Level/StageSelect/StageSelect.StageSelect"))))

(fn `UserConstructionScript`
  (`parent.UserConstructionScript`))