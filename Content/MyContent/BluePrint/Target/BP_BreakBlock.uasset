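; BP_BreakBlock is a destructible target block that breaks when a BP_Ball hits it fast enough.
; On hit, ball speed above Resist triggers Gimmick, applies strong directional damage to the Destructible, clears CanTarget and plays a bomb sound.
; On fracture it spawns an explosion, disables collision, then a Fade timeline drives the material alpha parameter before the actor is destroyed.
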(event `self.Destructible.OnComponentHit`
  (params (HitComponent :type "PrimitiveComponent Object Reference") (OtherActor :type "Actor Object Reference") (OtherComp :type "PrimitiveComponent Object Reference") (NormalImpulse :type "Vector Structure") (Hit :type "HitResult Structure (by ref)"))
  (bind _destructible (`self.Destructible`))
  (bind _returnvalue (`SceneComponent.K2_GetComponentLocation` _destructible))
  (bind _asbp_ball (cast `/Game/MyContent/BluePrint/BP_Ball` OtherActor))
  (bind _sphere (`/Game/MyContent/BluePrint/BP_Ball.Sphere` _asbp_ball))
  (bind _returnvalue_2 (`PrimitiveComponent.GetPhysicsLinearVelocity` _sphere "None"))
  (if (> (`KismetMathLibrary.VSize` _returnvalue_2) (`self.Resist`))
    (`self.Gimmick` true)
    (`DestructibleComponent.ApplyDamage` _destructible 1000.0 _returnvalue (`KismetMathLibrary.GetForwardVector` (`KismetMathLibrary.FindLookAtRotation` (`SceneComponent.K2_GetComponentLocation` _sphere) _returnvalue)) 50000.0)
    (set `self.CanTarget` false)
    (`GameplayStatics.PlaySoundAtLocation` "/Game/MyContent/Sounds/SE_Bomb.SE_Bomb" (`self.K2_GetActorLocation`) (struct) 1.0 1.0 0.0 null null null)))

(event `self.Destructible.OnComponentFracture`
  (params (HitPoint :type "Vector Structure (by ref)") (HitDirection :type "Vector Structure (by ref)"))
  (bind (_returnvalue_location _returnvalue_rotation _returnvalue_scale) (`KismetMathLibrary.BreakTransform` (`self.GetTransform`)))
  (bind _destructible (`self.Destructible`))
  (`GameplayStatics.SpawnEmitterAtLocation` "/Game/StarterContent/Particles/P_Explosion.P_Explosion" _returnvalue_location _returnvalue_rotation (* _returnvalue_scale 10.0))
  (`PrimitiveComponent.SetCollisionEnabled` _destructible "NoCollision")
  (`PrimitiveComponent.CreateDynamicMaterialInstance` _destructible 0 "/Game/MyContent/Material/M_Debug.M_Debug" "None")
  (bind (_direction _alpha) (`Timeline|Fade`)
    (:`Update`
      (`MeshComponent.SetScalarParameterValueOnMaterials` _destructible "alpha" _alpha))
    (:`Finished`
      (`self.K2_DestroyActor`))))

(fn `UserConstructionScript`
  (`parent.UserConstructionScript`))